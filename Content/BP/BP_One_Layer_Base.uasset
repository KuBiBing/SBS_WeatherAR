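; BP_One_Layer_Base displays an image layer over a base map on OverlayMesh, optionally animated as a frame sequence.
; The construction script sets the overlay texture on a dynamic material, with UV offset and scale derived from overlay and base latitude/longitude bounds.
; With EnableAnimation, BeginPlay imports IMAGEDIRECTORY files at runtime into TEXTUREARRAY.
; A timeline scaled to PLAYTIMESEC then indexes that array to swap overlay textures, reapplying the UV placement each update.
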(event `LoadComplete`
  (bind _overlay_min_lng (`self.OVERLAY_MIN_LNG`))
  (bind _base_max_lat (`self.BASE_MAX_LAT`))
  (bind _base_min_lat (`self.BASE_MIN_LAT`))
  (bind _base_max_lng (`self.BASE_MAX_LNG`))
  (bind _base_min_lng (`self.BASE_MIN_LNG`))
  (bind _overlay_max_lat (`self.OVERLAY_MAX_LAT`))
  (`KismetSystemLibrary.PrintString` "load complete!")
  (`TimelineComponent.SetPlayRate` (`self.타임라인`) (/ 1.0 (`self.PLAY_TIME_SEC`)))
  (bind (_direction `_노멀타임라인`) (`Timeline|타임라인`)
    (:`Update`
      (`MaterialInstanceDynamic.SetTextureParameterValue` (stale `self.ReceiveBeginPlay` _returnvalue) "T_Overlay" (`|GetArrayItem` (`self._TEXTURE_ARRAY`) (`KismetMathLibrary.FFloor` (* `_노멀타임라인` (`KismetArrayLibrary.Array_Length` (`self._TEXTURE_ARRAY`))))) :!label _label)
      ;[1 1 1] XY offset, scale을 머티리얼의 변수(Overlay_U_Offset 등)로 적용
      (`MaterialInstanceDynamic.SetScalarParameterValue` (stale `self.ReceiveBeginPlay` _returnvalue) "Overlay_U_Offset" (/ (- _overlay_min_lng _base_min_lng) (- _base_max_lng _base_min_lng)))
      (`MaterialInstanceDynamic.SetScalarParameterValue` (stale `self.ReceiveBeginPlay` _returnvalue) "Overlay_V_Offset" (/ (- _base_max_lat _overlay_max_lat) (- _base_max_lat _base_min_lat)))
      (`MaterialInstanceDynamic.SetScalarParameterValue` (stale `self.ReceiveBeginPlay` _returnvalue) "Overlay_U_Scale" (/ (- (`self.OVERLAY_MAX_LNG`) _overlay_min_lng) (- _base_max_lng _base_min_lng)))
      (`MaterialInstanceDynamic.SetScalarParameterValue` (stale `self.ReceiveBeginPlay` _returnvalue) "Overlay_V_Scale" (/ (- _overlay_max_lat (`self.OVERLAY_MIN_LAT`)) (- _base_max_lat _base_min_lat))))))

(event `self.ReceiveBeginPlay`
  (if (`self.EnableAnimation`)
    (`|ExecutionSequence`
      (:`then_0`
        (bind _returnvalue (`PrimitiveComponent.CreateDynamicMaterialInstance` (`self.OverlayMesh`) 0 null "None"))
        (goto _label))
      (:`then_1`
        (bind (_textures _filenames) (`self.Read Directory` (`self.IMAGE_DIRECTORY`)))
        (set `self._IMAGE_NAMES` _filenames)
        (`self.LoadComplete`)))))

(fn `AppendString`
  (params (NewParam :type String))
  (returns (NewParam1 :type String))
  (return (`KismetStringLibrary.Concat_StrStr` NewParam "in Function")))

(fn `Read Directory`
  (params (Directory :type String))
  (returns (Textures :type "Array of Texture2D Object Reference") (FileNames :type "Array of String"))
  (bind _foundfiles (`BlueprintFileUtilsBPLibrary.FindFiles` Directory))
  (for _array_element _foundfiles
    (bind _returnvalue (`KismetRenderingLibrary.ImportFileAsTexture2D` (`KismetStringLibrary.Concat_StrStr` (`KismetStringLibrary.Concat_StrStr` Directory "/") _array_element)))
    (`KismetArrayLibrary.Array_Add` (`self._TEXTURE_ARRAY`) _returnvalue))
  (return _ _foundfiles))

(fn `UserConstructionScript`
  (bind _overlay_min_lng (`self.OVERLAY_MIN_LNG`))
  (bind _base_max_lat (`self.BASE_MAX_LAT`))
  (bind _base_min_lat (`self.BASE_MIN_LAT`))
  (bind _base_max_lng (`self.BASE_MAX_LNG`))
  (bind _base_min_lng (`self.BASE_MIN_LNG`))
  (bind _overlay_max_lat (`self.OVERLAY_MAX_LAT`))
  (bind _returnvalue (`PrimitiveComponent.CreateDynamicMaterialInstance` (`self.OverlayMesh`) 0 null "None"))
  ;[1 1 1] XY offset, scale을 머티리얼의 변수(Overlay_U_Offset 등)로 적용
  (`MaterialInstanceDynamic.SetScalarParameterValue` _returnvalue "Overlay_U_Offset" (/ (- _overlay_min_lng _base_min_lng) (- _base_max_lng _base_min_lng)))
  (`MaterialInstanceDynamic.SetScalarParameterValue` _returnvalue "Overlay_V_Offset" (/ (- _base_max_lat _overlay_max_lat) (- _base_max_lat _base_min_lat)))
  (`MaterialInstanceDynamic.SetScalarParameterValue` _returnvalue "Overlay_U_Scale" (/ (- (`self.OVERLAY_MAX_LNG`) _overlay_min_lng) (- _base_max_lng _base_min_lng)))
  (`MaterialInstanceDynamic.SetScalarParameterValue` _returnvalue "Overlay_V_Scale" (/ (- _overlay_max_lat (`self.OVERLAY_MIN_LAT`)) (- _base_max_lat _base_min_lat)))
  (`MaterialInstanceDynamic.SetTextureParameterValue` _returnvalue "T_BaseMap" null)
  (`MaterialInstanceDynamic.SetTextureParameterValue` _returnvalue "T_Overlay" (`self.OverlayTexture`)))