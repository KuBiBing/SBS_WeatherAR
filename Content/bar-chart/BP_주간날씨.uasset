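; Weekly weather (주간날씨) display Blueprint that presents a day's forecast through text components and an icon.
; On BeginPlay it fills the day number, day of week, additional info, icon info and high and low temperature texts from the T날씨 weather data.
; It also sets the child actor class of the icon component, with no later updates and an empty construction script.
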(event `self.ReceiveBeginPlay`
  (bind `_t_날씨` (`self.T_날씨`))
  (`Text3DComponent.SetText` (`self.day number-comp`) `_t_날씨`)
  (`Text3DComponent.SetText` (`self.day of week-comp`) `_t_날씨`)
  (`Text3DComponent.SetText` (`self.day add info-comp`) `_t_날씨`)
  (`Text3DComponent.SetText` (`self.icon-solo-add info`) `_t_날씨`)
  (`ChildActorComponent.SetChildActorClass` (`self.Icon-solo`) null)
  (`Text3DComponent.SetText` (`self.Temp-high`) `_t_날씨`)
  (`Text3DComponent.SetText` (`self.Temp-low`) `_t_날씨`))

(fn `UserConstructionScript`)